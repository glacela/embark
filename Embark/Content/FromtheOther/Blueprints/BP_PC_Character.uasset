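; BP_PC_Character is a dog player character with appearance customization and a manually rotated camera.
; Enhanced Input adds a camera mapping context on BeginPlay, and left/right actions yaw the SpringArm in fixed steps, printing debug text.
; Customization events swap breed meshes (animation class only for Shiba and Chihuahua), show one class child component, and set fur and pattern material parameters.
; The construction script makes Knight and Mage components follow the body's pose.
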(event Input|EnhancedActionEvents|EnhancedInputActionIA_TurnCameraL
  (params (ActionValue :type Boolean) (ElapsedSeconds :type Float%20%28double-precision%29) (TriggeredSeconds :type Float%20%28double-precision%29) (InputAction :type Input%20Action%20Object%20Reference :default "/Game/FromtheOther/Blueprints/IA_TurnCameraL.IA_TurnCameraL"))
  (:Triggered
    (if true :!label _label
      (Transformation|AddRelativeRotation (Variables|Default|GetSpringArm) (Math|Conversions|RotationFromXVector (Class|KismetMathLibrary|CreateVectorfromYawPitch 1.0 0.0 1.0)) false false)
      (Development|PrintString "Is triggered")))
  (:Ongoing
    (goto _label)))

(event Input|EnhancedActionEvents|EnhancedInputActionIA_TurnCameraR
  (params (ActionValue :type Boolean) (ElapsedSeconds :type Float%20%28double-precision%29) (TriggeredSeconds :type Float%20%28double-precision%29) (InputAction :type Input%20Action%20Object%20Reference :default "/Game/FromtheOther/Blueprints/IA_TurnCameraR.IA_TurnCameraR"))
  (:Triggered
    (if true :!label _label
      (Transformation|AddRelativeRotation (Variables|Default|GetSpringArm) (Math|Conversions|RotationFromXVector (Class|KismetMathLibrary|CreateVectorfromYawPitch -1.0 0.0 1.0)) false false)
      (Development|PrintString "Is triggered")))
  (:Ongoing
    (goto _label)))

(event EventBeginPlay
  (bind _asplayer_controller (Utilities|Casting|CastToPlayerController (Pawn|GetController)))
  (Utilities|IsValid (PlayerController|LocalPlayerSubsystems|GetEnhancedInputLocalPlayerSubsystem _asplayer_controller)
    (:Is%20Valid
      (Input|AddMappingContext (PlayerController|LocalPlayerSubsystems|GetEnhancedInputLocalPlayerSubsystem _asplayer_controller) "/Game/FromtheOther/Blueprints/MC_CameraRotation.MC_CameraRotation" 1 "(bIgnoreAllPressedKeysUntilRelease=True,bForceImmediately=False,bNotifyUserSettings=False)"))))

(event Custom|Set%20Breed
  (params (Breed%20Index :type Integer))
  (bind _mesh (Variables|Character|GetMesh))
  (switch int Breed%20Index
    (:Default
      (Components|SkeletalMesh|SetSkeletalMeshAsset _mesh "/Game/FromtheOther/Characters/PC/PC_Shiba_Rig.PC_Shiba_Rig" :!label _label)
      (Components|Animation|SetAnimationMode _mesh "AnimationBlueprint" true)
      (Class|SkeletalMeshComponent|SetAnimClass _mesh "/Game/FromtheOther/Blueprints/ABP_Shiba.ABP_Shiba_C"))
    (:0
      (goto _label))
    (:1
      (Components|SkeletalMesh|SetSkeletalMeshAsset _mesh "/Game/FromtheOther/Characters/PC/PC_Basque_Rig.PC_Basque_Rig"))
    (:2
      (Components|SkeletalMesh|SetSkeletalMeshAsset _mesh "/Game/FromtheOther/Characters/PC/PC_Chihuahua_Rig.PC_Chihuahua_Rig")
      (Components|Animation|SetAnimationMode _mesh "AnimationBlueprint" true)
      (Class|SkeletalMeshComponent|SetAnimClass _mesh "/Game/FromtheOther/Blueprints/ABP_Chihuahua.ABP_Chihuahua_C"))))

(event Custom|Set%20Class
  (params (Class%20Index :type Integer))
  (bind _mesh (Variables|Character|GetMesh))
  (bind _children (Components|GetChildrenComponents _mesh false))
  (Rendering|SetVisibility _children false false)
  (Rendering|SetVisibility (Utilities|Array|Get(acopy) _children Class%20Index) true false))

(event Custom|Set%20Pattern%20Style
  (params (Value :type Texture%20Object%20Reference) (ParameterName :type Name))
  (bind _returnvalue (Rendering|Material|CreateDynamicMaterialInstance (Variables|Character|GetMesh) 4 0 "None" :!class /Script/Engine.PrimitiveComponent))
  (Rendering|Material|SetTextureParameterValue _returnvalue ParameterName Value))

(event Custom|Set%20Fur%20Color
  (params (Value :type Texture%20Object%20Reference))
  (bind _returnvalue (Rendering|Material|CreateDynamicMaterialInstance (Variables|Character|GetMesh) 4 0 "None" :!class /Script/Engine.PrimitiveComponent))
  (Rendering|Material|SetTextureParameterValue _returnvalue "ParamFurColor" Value))

(event Custom|Set%20Pattern%20Color
  (params (Value :type Texture%20Object%20Reference) (ParameterName :type Name))
  (bind _returnvalue (Rendering|Material|CreateDynamicMaterialInstance (Variables|Character|GetMesh) 4 0 "None" :!class /Script/Engine.PrimitiveComponent))
  (Rendering|Material|SetTextureParameterValue _returnvalue ParameterName Value))

(event Custom|Set%20Pattern%20Intensity
  (params (ParameterValue :type Float%20%28single-precision%29) (ParameterName :type Name))
  (Rendering|Material|SetScalarParameterValueonMaterials (Variables|Character|GetMesh) ParameterName ParameterValue))

(fn ConstructionScript
  (Components|SkinnedMesh|SetLeaderPoseComponent (Variables|Default|GetClass_Knight) (Variables|Character|GetMesh) false false))