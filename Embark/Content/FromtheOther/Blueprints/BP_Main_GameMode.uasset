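; BP_Main_GameMode is the gameplay game mode that adds the gameplay UI and sets up the player character on BeginPlay.
; Set_PC copies breed, fur color, pattern color, pattern style and class from GI_Main onto the first BP_PC_Character found in the level.
; BeginPlay also prints the saved character name and each stat as debug output.
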(event Custom|Set_PC
  (Utilities|FlowControl|Sequence
    (:then_0
      (bind _asgi_main (Utilities|Casting|CastToGI_Main (Game|GetGameInstance))))
    (:then_1
      (bind _outactors (Actor|GetAllActorsOfClass "/Game/FromtheOther/Blueprints/BP_PC_Character.BP_PC_Character_C"))
      (bind _asbp_pc_character (Utilities|Casting|CastToBP_PC_Character (Utilities|Array|Get(acopy) _outactors))))
    (:then_2
      (Default|SetBreed _asbp_pc_character (Variables|/Game/FromtheOther/Blueprints/GI_Main.GI_Main_C|GetPC_Breed _asgi_main))
      (Default|SetFurColor _asbp_pc_character (Variables|/Game/FromtheOther/Blueprints/GI_Main.GI_Main_C|GetPC_FurColor _asgi_main))
      (Default|SetPatternColor _asbp_pc_character (Variables|/Game/FromtheOther/Blueprints/GI_Main.GI_Main_C|GetPC_FurPatternColor _asgi_main))
      (Default|SetPatternStyle _asbp_pc_character (Variables|/Game/FromtheOther/Blueprints/GI_Main.GI_Main_C|GetPC_FurPattern _asgi_main))
      (Default|SetClass _asbp_pc_character (Variables|/Game/FromtheOther/Blueprints/GI_Main.GI_Main_C|GetPC_Class _asgi_main)))))

(event EventBeginPlay
  (Utilities|FlowControl|Sequence
    (:then_0
      (bind _returnvalue (UserInterface|CreateWidget "/Game/FromtheOther/Blueprints/Widgets/WBP_Gameplay_UI.WBP_Gameplay_UI_C"))
      (UserInterface|Viewport|AddtoViewport _returnvalue 0))
    (:then_1
      (CallFunction|SetPC)
      (bind _asgi_main (Utilities|Casting|CastToGI_Main (Game|GetGameInstance)))
      (Development|PrintString "Your name is:")
      (Development|PrintString (Utilities|String|ToString(Text) (Variables|/Game/FromtheOther/Blueprints/GI_Main.GI_Main_C|GetPC_Name _asgi_main)))
      (for _array_element (Variables|/Game/FromtheOther/Blueprints/GI_Main.GI_Main_C|GetPC_Stats _asgi_main)
        (Development|PrintString (Utilities|String|ToString(Integer) _array_element))))))

(event EventTick
  (params (DeltaSeconds :type Float%20%28single-precision%29)))

(fn ConstructionScript)