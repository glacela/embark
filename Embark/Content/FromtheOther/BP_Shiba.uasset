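; BP_Shiba is a customizable character Blueprint with switchable breeds, Knight and Mage class meshes, and stored, debug-printed stats.
; SetBreed swaps visibility between breed meshes indexed under the root and makes the new one the leader pose for both class meshes.
; Pattern, fur color and pattern color events set texture parameters through dynamic material instances on every root child skinned mesh.
; The construction script links class meshes to the VarBreedIndex mesh and hides it.
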(event Custom|SetPatternColor
  (params (Value :type Texture%20Object%20Reference))
  ;[1 1 1] Set Pattern Color on all Breeds
  (for _array_element (Components|GetChildrenComponents (Variables|Default|GetDefaultSceneRoot) false)
    (bind _asskinned_mesh_component (Utilities|Casting|CastToSkinnedMeshComponent _array_element))
    (bind _returnvalue (Rendering|Material|CreateDynamicMaterialInstance _asskinned_mesh_component 0 0 "None" :!class /Script/Engine.PrimitiveComponent))
    (Rendering|Material|SetTextureParameterValue _returnvalue "ParamPatternColor" Value)))

(event Custom|SetPatternStyle
  (params (Value :type Texture%20Object%20Reference))
  ;[1 1 1] Set Pattern Style on all Breeds
  (for _array_element (Components|GetChildrenComponents (Variables|Default|GetDefaultSceneRoot) false)
    (bind _asskinned_mesh_component (Utilities|Casting|CastToSkinnedMeshComponent _array_element))
    (bind _returnvalue (Rendering|Material|CreateDynamicMaterialInstance _asskinned_mesh_component 0 0 "None" :!class /Script/Engine.PrimitiveComponent))
    (Rendering|Material|SetTextureParameterValue _returnvalue "ParamPattern" Value)))

(event Custom|SetFurColor
  (params (Value :type Texture%20Object%20Reference))
  ;[1 1 1] Set Fur Color on all Breeds
  (for _array_element (Components|GetChildrenComponents (Variables|Default|GetDefaultSceneRoot) false)
    (bind _asskinned_mesh_component (Utilities|Casting|CastToSkinnedMeshComponent _array_element))
    (bind _returnvalue (Rendering|Material|CreateDynamicMaterialInstance _asskinned_mesh_component 0 0 "None" :!class /Script/Engine.PrimitiveComponent))
    (Rendering|Material|SetTextureParameterValue _returnvalue "ParamFurColor" Value)))

(event Custom|SetClassKnight
  (Rendering|SetVisibility (Variables|Default|GetSkelMage) false false)
  (Rendering|SetVisibility (Variables|Default|GetSkelKnight) true false))

(event Custom|SetClassMage
  (Rendering|SetVisibility (Variables|Default|GetSkelKnight) false false)
  (Rendering|SetVisibility (Variables|Default|GetSkelMage) true false))

(event Custom|Set%20Breed
  (params (ParamPrevBreed :type Integer) (ParamNewBreed :type Integer))
  (bind _asskinned_mesh_component (Utilities|Casting|CastToSkinnedMeshComponent (Components|GetChildComponent (Variables|Default|GetDefaultSceneRoot) ParamPrevBreed)))
  (Rendering|SetVisibility _asskinned_mesh_component false false)
  (bind _asskinned_mesh_component_2 (Utilities|Casting|CastToSkinnedMeshComponent (Components|GetChildComponent (Variables|Default|GetDefaultSceneRoot) ParamNewBreed)))
  (Components|SkinnedMesh|SetLeaderPoseComponent (Variables|Default|GetSkelMage) _asskinned_mesh_component_2 false false)
  (Rendering|SetVisibility _asskinned_mesh_component_2 true false))

(event Custom|Set%20PC%20Stats
  (params (PC%20stats :type Array%20of%20Integers))
  (bind _output_get (Variables|Default|SetPCstats PC%20stats))
  (for _array_element _output_get
    (Development|PrintString (Utilities|String|ToString(Integer) _array_element))))

(fn ConstructionScript
  (bind _asskinned_mesh_component (Utilities|Casting|CastToSkinnedMeshComponent (Components|GetChildComponent (Variables|Default|GetDefaultSceneRoot) (Variables|Default|GetVarBreedIndex))))
  (Components|SkinnedMesh|SetLeaderPoseComponent (Variables|Default|GetSkelMage) _asskinned_mesh_component false false)
  (Rendering|SetVisibility _asskinned_mesh_component false false))