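; BP_PlayerController is a player controller that shows the mouse cursor on BeginPlay.
; An unconnected chain sketches click-to-move but never runs, as no event triggers it.
; That chain deprojects the cursor into a debug-drawn Visibility line trace and, on a hit, passes the location to SimpleMoveToLocation.
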(event EventBeginPlay
  (Variables|/Script/Engine.PlayerController|SetbShowMouseCursor (Game|GetPlayerController 0) true))

(fn ConstructionScript)