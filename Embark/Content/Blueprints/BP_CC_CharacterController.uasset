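; BP_CC_CharacterController handles the Embark event, preparing the player character and capturing a profile picture of it.
; Embark finds the first BP_PC_Character, resets its rotation to zero, then triggers a one-shot SceneCaptureProfile capture, printing debug strings along the way.
; The nodes that create and display WBP_Gameplay_UI are disconnected, so no overlay opens despite the graph comment.
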(event Custom|Event%20Embark
  ;[1 1 1] Resets PC Rotation, Takes a Pic and opens the Porfile Pic Testing Overlay
  (Utilities|FlowControl|Sequence
    (:then_0
      (bind _outactors (Actor|GetAllActorsOfClass "/Game/Blueprints/BP_PC_Character.BP_PC_Character_C"))
      (bind _asbp_pc_character (Utilities|Casting|CastToBP_PC_Character (Utilities|Array|Get(acopy) _outactors)))
      (Transformation|SetActorRotation _asbp_pc_character)
      (Development|PrintString "ROTATION"))
    (:then_1
      (Rendering|SceneCapture|CaptureScene (Variables|Default|GetSceneCapture_Profile) :!class /Script/Engine.SceneCaptureComponent2D)
      (Development|PrintString "TAKE PIC"))))

(fn ConstructionScript)