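; Main game mode that sets up each scene based on the SceneIndex stored in GI_Main.
; BeginPlay adds the main menu, character creation or gameplay UI widget, respawning the player at a named PlayerStart for the latter two.
; In gameplay, Set_PC copies saved breed, fur, pattern and class choices from the game instance onto the first BP_PC_Character found.
; It also prints the character's name and stats to screen.
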(event Custom|Set_PC
  (Utilities|FlowControl|Sequence
    (:then_0
      (bind _asgi_main (Utilities|Casting|CastToGI_Main (Game|GetGameInstance))))
    (:then_1
      (bind _outactors (Actor|GetAllActorsOfClass "/Game/Blueprints/BP_PC_Character.BP_PC_Character_C"))
      (bind _asbp_pc_character (Utilities|Casting|CastToBP_PC_Character (Utilities|Array|Get(acopy) _outactors))))
    (:then_2
      (Default|SetBreed _asbp_pc_character (Variables|/Game/Blueprints/GI_Main.GI_Main_C|GetPC_Breed _asgi_main))
      (Default|SetFurColor _asbp_pc_character (Variables|/Game/Blueprints/GI_Main.GI_Main_C|GetPC_FurColor _asgi_main))
      (Default|SetPatternColor _asbp_pc_character (Variables|/Game/Blueprints/GI_Main.GI_Main_C|GetPC_FurPatternColor _asgi_main) "None")
      (Default|SetPatternStyle _asbp_pc_character (Variables|/Game/Blueprints/GI_Main.GI_Main_C|GetPC_FurPattern _asgi_main) "None")
      (Default|SetClass _asbp_pc_character (Variables|/Game/Blueprints/GI_Main.GI_Main_C|GetPC_Class _asgi_main)))))

(event EventBeginPlay
  (bind _returnvalue (Game|GetPlayerController 0))
  (bind _returnvalue_2 (Game|GetPlayerController 0))
  (bind _asgi_main (Utilities|Casting|CastToGI_Main (Game|GetGameInstance)))
  (switch int (Variables|/Game/Blueprints/GI_Main.GI_Main_C|GetSceneIndex _asgi_main)
    (:0
      (bind _returnvalue_3 (UserInterface|CreateWidget "/Game/Blueprints/Widgets/WBP_MainMenu.WBP_MainMenu_C"))
      (UserInterface|Viewport|AddtoViewport _returnvalue_3 0))
    (:1
      (bind _returnvalue_4 (UserInterface|CreateWidget "/Game/Blueprints/Widgets/WBP_CC_Code.WBP_CC_Code_C"))
      (UserInterface|Viewport|AddtoViewport _returnvalue_4 0)
      (Class|GameModeBase|RestartPlayeratPlayerStart _returnvalue_2 (Class|GameModeBase|FindPlayerStart _returnvalue_2 "PS_CC")))
    (:2
      (Utilities|FlowControl|Sequence
        (:then_0
          (bind _returnvalue_5 (UserInterface|CreateWidget "/Game/Blueprints/Widgets/WBP_Gameplay_UI.WBP_Gameplay_UI_C"))
          (UserInterface|Viewport|AddtoViewport _returnvalue_5 0))
        (:then_1
          (Class|GameModeBase|RestartPlayeratPlayerStart _returnvalue (Class|GameModeBase|FindPlayerStart _returnvalue "PS_Game"))
          (CallFunction|SetPC)
          (bind _asgi_main_2 (Utilities|Casting|CastToGI_Main (Game|GetGameInstance)))
          (Development|PrintString "Your name is:")
          (Development|PrintString (Utilities|String|ToString(Text) (Variables|/Game/Blueprints/GI_Main.GI_Main_C|GetPC_Name _asgi_main_2)))
          (for _array_element (Variables|/Game/Blueprints/GI_Main.GI_Main_C|GetPC_Stats _asgi_main_2)
            (Development|PrintString (Utilities|String|ToString(Integer) _array_element))))))))

(fn ConstructionScript)